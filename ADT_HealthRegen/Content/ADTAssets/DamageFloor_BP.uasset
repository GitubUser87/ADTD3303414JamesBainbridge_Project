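; Damage floor actor that hurts the player character while they stand inside its Box trigger.
; Overlap begin sets an On flag and applies a fixed damage immediately, then repeats it through a short Delay loop until overlap end clears the flag.
; Only player 0's character triggers it or takes damage; other actors are ignored.
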(event OnComponentBeginOverlap(Box)
  (params (OverlappedComponent :type Primitive%20Component%20Object%20Reference) (OtherActor :type Actor%20Object%20Reference) (OtherComp :type Primitive%20Component%20Object%20Reference) (OtherBodyIndex :type Integer) (bFromSweep :type Boolean) (SweepResult :type Hit%20Result%20Structure%20%28by%20ref%29))
  (bind _returnvalue (Game|GetPlayerCharacter 0))
  ;[0.15 0.15 0.15 0.5] Apply damage
  (if (== OtherActor _returnvalue)
    (Variables|Default|SetOn? true)
    (Game|Damage|ApplyDamage _returnvalue 1e+01 0 0 :!label _label)
    (Utilities|FlowControl|Delay 0.2)
    (if (Variables|Default|GetOn?)
      (goto _label))))

(event OnComponentEndOverlap(Box)
  (params (OverlappedComponent :type Primitive%20Component%20Object%20Reference) (OtherActor :type Actor%20Object%20Reference) (OtherComp :type Primitive%20Component%20Object%20Reference) (OtherBodyIndex :type Integer))
  ;[0.15 0.15 0.15 0.5] Apply damage
  (if (== OtherActor (Game|GetPlayerCharacter 0))
    (Variables|Default|SetOn? false)))

(fn ConstructionScript)