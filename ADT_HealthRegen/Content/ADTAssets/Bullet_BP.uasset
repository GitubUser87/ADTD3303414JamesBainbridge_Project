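; Bullet actor that damages the player on contact and destroys itself five seconds after spawning.
; Its sphere overlap checks for the player character, applies fixed damage, decrements PointsEarned on an Enemy reference and prints the new value.
; The overlap does not destroy the bullet, so only the timer removes it.
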(event OnComponentBeginOverlap(Sphere)
  (params (OverlappedComponent :type Primitive%20Component%20Object%20Reference) (OtherActor :type Actor%20Object%20Reference) (OtherComp :type Primitive%20Component%20Object%20Reference) (OtherBodyIndex :type Integer) (bFromSweep :type Boolean) (SweepResult :type Hit%20Result%20Structure%20%28by%20ref%29))
  (bind _returnvalue (Game|GetPlayerCharacter 0))
  ;[0.15 0.15 0.15 0.5] Deal Damage
  (if (== OtherActor _returnvalue)
    (Game|Damage|ApplyDamage _returnvalue 5.0 0 0)
    (bind _result (Math|Integer|DecrementInt (Variables|/Game/ADTAssets/Enemy_BP.Enemy_BP_C|GetPoints%20Earned (Variables|Default|Getenemy)))
      (:%20%20
        (Development|PrintString (Utilities|String|ToString(Integer) _result))))))

(event EventBeginPlay
  ;[0.15 0.15 0.15 0.5] Self Destruct
  (Utilities|FlowControl|Delay 5.0)
  (Actor|DestroyActor))

(fn ConstructionScript)