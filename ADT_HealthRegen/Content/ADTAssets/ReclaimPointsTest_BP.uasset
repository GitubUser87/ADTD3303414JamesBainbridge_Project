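; Test pickup Blueprint that restores points to the player character on overlap.
; When player 0 overlaps the RegainPoints component, it casts to BP_ThirdPersonCharacter and adds EarnPoints to CurrentPoints, clamped between zero and MaxPoints as an integer.
; The add is skipped only at a hardcoded 100 rather than MaxPoints, and the actor is not destroyed afterwards, so each new overlap can award again.
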(event OnComponentBeginOverlap(RegainPoints)
  (params (OverlappedComponent :type Primitive%20Component%20Object%20Reference) (OtherActor :type Actor%20Object%20Reference) (OtherComp :type Primitive%20Component%20Object%20Reference) (OtherBodyIndex :type Integer) (bFromSweep :type Boolean) (SweepResult :type Hit%20Result%20Structure%20%28by%20ref%29))
  (bind _returnvalue (Game|GetPlayerCharacter 0))
  ;[0.15 0.15 0.15 0.5] Add Points
  (if (== OtherActor _returnvalue)
    (bind _asbp_third_person_character (Utilities|Casting|CastToBP_ThirdPersonCharacter _returnvalue))
    (if (!= (Variables|/Game/ThirdPerson/Blueprints/BP_ThirdPersonCharacter.BP_ThirdPersonCharacter_C|GetCurrentPoints _asbp_third_person_character) 100)
      (Variables|/Game/ThirdPerson/Blueprints/BP_ThirdPersonCharacter.BP_ThirdPersonCharacter_C|SetCurrentPoints _asbp_third_person_character (Math|Conversions|ToFloat(Integer) (Math|Integer|Clamp(Integer) (+ (Variables|/Game/ThirdPerson/Blueprints/BP_ThirdPersonCharacter.BP_ThirdPersonCharacter_C|GetCurrentPoints _asbp_third_person_character) (Variables|Default|GetEarnPoints)) 0 (Math|Float|Truncate (Variables|/Game/ThirdPerson/Blueprints/BP_ThirdPersonCharacter.BP_ThirdPersonCharacter_C|GetMaxPoints _asbp_third_person_character))))))))

(fn ConstructionScript)