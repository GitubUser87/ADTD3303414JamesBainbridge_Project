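; CheckPoint_BP is a checkpoint actor that saves the player's progress position and notifies linked enemy spawners.
; On BeginPlay it caches the player's BP_ThirdPersonCharacter.
; When the player overlaps its CheckPoint component, it writes that component's world location to the character's CheckPoint variable and prints a message.
; It then calls FunctionMessage on every EnemySpawn_BP carrying its Tag, with no guard against repeat triggering.
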(event OnComponentBeginOverlap(CheckPoint)
  (params (OverlappedComponent :type Primitive%20Component%20Object%20Reference) (OtherActor :type Actor%20Object%20Reference) (OtherComp :type Primitive%20Component%20Object%20Reference) (OtherBodyIndex :type Integer) (bFromSweep :type Boolean) (SweepResult :type Hit%20Result%20Structure%20%28by%20ref%29))
  ;[0.15 0.15 0.15 0.5] 'Kill'Player
  (if (== OtherActor (Game|GetPlayerCharacter 0))
    (Development|PrintString "CheckPoint Obtained")
    (Variables|/Game/ThirdPerson/Blueprints/BP_ThirdPersonCharacter.BP_ThirdPersonCharacter_C|SetCheckPoint (Variables|Default|GetCharREF) (Transformation|GetWorldLocation (Variables|Default|GetCheckPoint)))
    (bind _outactors (Actor|GetAllActorsOfClasswithTag "/Game/ADTAssets/Enemies/EnemySpawn_BP.EnemySpawn_BP_C" (Variables|Default|GetTag)))
    (for _array_element _outactors
      (Class|Function|Function(Message) _array_element))))

(event EventBeginPlay
  ;[0.15 0.15 0.15 0.5] Player REF
  (bind _asbp_third_person_character (Utilities|Casting|CastToBP_ThirdPersonCharacter (Game|GetPlayerCharacter 0)))
  (Variables|Default|SetCharREF _asbp_third_person_character))

(fn ConstructionScript)