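; ItemBoxMini_BP is a pickup actor that adds one item box to the player's count when touched, filed in an Unused folder.
; Its Trigger overlap checks for the player character, then runs once through a DoOnce gate.
; It increments ItemBoxes on BP_ThirdPersonCharacter, clamps the count between zero and ItemMax, and destroys itself.
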(event OnComponentBeginOverlap(Trigger)
  (params (OverlappedComponent :type Primitive%20Component%20Object%20Reference) (OtherActor :type Actor%20Object%20Reference) (OtherComp :type Primitive%20Component%20Object%20Reference) (OtherBodyIndex :type Integer) (bFromSweep :type Boolean) (SweepResult :type Hit%20Result%20Structure%20%28by%20ref%29))
  ;[0.15 0.15 0.15 0.5] ItemBox add to list
  (if (== OtherActor (Game|GetPlayerCharacter 0))
    (Utilities|FlowControl|DoOnce false
      (:Completed
        (bind _returnvalue (Actor|GetActorOfClass "/Game/ThirdPerson/Blueprints/BP_ThirdPersonCharacter.BP_ThirdPersonCharacter_C"))
        (bind _result (Math|Integer|IncrementInt (Variables|/Game/ThirdPerson/Blueprints/BP_ThirdPersonCharacter.BP_ThirdPersonCharacter_C|GetItemBoxes _returnvalue))
          (:%20%20
            (Variables|/Game/ThirdPerson/Blueprints/BP_ThirdPersonCharacter.BP_ThirdPersonCharacter_C|SetItemBoxes _returnvalue (Math|Integer|Clamp(Integer) _result 0 (Variables|/Game/ThirdPerson/Blueprints/BP_ThirdPersonCharacter.BP_ThirdPersonCharacter_C|GetItemMax _returnvalue)))
            (Actor|DestroyActor)))))))

(fn ConstructionScript)