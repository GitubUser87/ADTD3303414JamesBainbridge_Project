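; Collectible point pickup that adds to the player's score and respawns after being collected.
; When the player overlaps the Box, it hides the Shape, plays a sound and increments PointsScore on the first CountdownPoints_BP widget found.
; Leaving the Box disables pickup via CanPickUp for a short delay, then re-enables it and shows the Shape again.
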(event OnComponentBeginOverlap(Box)
  (params (OverlappedComponent :type Primitive%20Component%20Object%20Reference) (OtherActor :type Actor%20Object%20Reference) (OtherComp :type Primitive%20Component%20Object%20Reference) (OtherBodyIndex :type Integer) (bFromSweep :type Boolean) (SweepResult :type Hit%20Result%20Structure%20%28by%20ref%29))
  ;[0.15 0.15 0.15 0.5] Pickup/turn off
  (if (and (== OtherActor (Game|GetPlayerCharacter 0)) (Variables|Default|GetCanPickUp?))
    (Rendering|SetVisibility (Variables|Default|GetShape) false false)
    (bind _foundwidgets (Widget|GetAllWidgetsOfClass "/Game/ADTAssets/Points/Unused/CountdownPoints_BP.CountdownPoints_BP_C" true))
    (Variables|/Game/ADTAssets/Points/Unused/CountdownPoints_BP.CountdownPoints_BP_C|SetPointsScore (Utilities|Array|Get(acopy) _foundwidgets) (+ (Variables|/Game/ADTAssets/Points/Unused/CountdownPoints_BP.CountdownPoints_BP_C|GetPointsScore (Utilities|Array|Get(acopy) _foundwidgets)) 1))
    (Audio|PlaySound2D "/Engine/VREditor/Sounds/UI/Dockable_Window_Pick_Up.Dockable_Window_Pick_Up" 1.0 1.0 0.0 0 0)))

(event OnComponentEndOverlap(Box)
  (params (OverlappedComponent :type Primitive%20Component%20Object%20Reference) (OtherActor :type Actor%20Object%20Reference) (OtherComp :type Primitive%20Component%20Object%20Reference) (OtherBodyIndex :type Integer))
  ;[0.15 0.15 0.15 0.5] Pickup/turn off
  (if (== OtherActor (Game|GetPlayerCharacter 0))
    (Variables|Default|SetCanPickUp? false)
    (Utilities|FlowControl|Delay 1.0)
    (Variables|Default|SetCanPickUp? true)
    (Rendering|SetVisibility (Variables|Default|GetShape) true false)))

(fn ConstructionScript)