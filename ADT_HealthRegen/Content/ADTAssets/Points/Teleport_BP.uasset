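; Teleport trigger actor that moves the player to a set location while their points are not yet at the maximum.
; It caches the third-person character at BeginPlay, then checks its current against maximum points when the player overlaps the trigger.
; On the first qualifying overlap only, via DoOnce, it adds a countdown points widget to the viewport and teleports the player to NewLocation.
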(event OnComponentBeginOverlap(Trigger)
  (params (OverlappedComponent :type Primitive%20Component%20Object%20Reference) (OtherActor :type Actor%20Object%20Reference) (OtherComp :type Primitive%20Component%20Object%20Reference) (OtherBodyIndex :type Integer) (bFromSweep :type Boolean) (SweepResult :type Hit%20Result%20Structure%20%28by%20ref%29))
  (bind _playerref (Variables|Default|GetPlayerRef))
  ;[0.15 0.15 0.15 0.5] Teleport + open widget
  (if (== OtherActor (Game|GetPlayerCharacter 0))
    (if (!= (Variables|/Game/ThirdPerson/Blueprints/BP_ThirdPersonCharacter.BP_ThirdPersonCharacter_C|GetCurrentPoints _playerref) (Variables|/Game/ThirdPerson/Blueprints/BP_ThirdPersonCharacter.BP_ThirdPersonCharacter_C|GetMaxPoints _playerref))
      (Utilities|FlowControl|DoOnce false
        (:Completed
          (bind _returnvalue (UserInterface|CreateWidget "/Game/ADTAssets/Points/CountdownPoints_BP.CountdownPoints_BP_C"))
          (UserInterface|Viewport|AddtoViewport _returnvalue 0)
          (Transformation|SetActorLocation (Game|GetPlayerCharacter 0) (Variables|Default|GetNew%20Location) false true))))))

(event EventBeginPlay
  ;[0.15 0.15 0.15 0.5] Player Ref
  (bind _asbp_third_person_character (Utilities|Casting|CastToBP_ThirdPersonCharacter (Game|GetPlayerCharacter 0)))
  (Variables|Default|SetPlayerRef _asbp_third_person_character))

(fn ConstructionScript)