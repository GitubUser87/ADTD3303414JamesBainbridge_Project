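; PointsBase_BP is a respawning points pickup for the third-person player character.
; When the player overlaps the Box while pickup is allowed, it hides the Shape, adds CustomScore to the character's CurrentPoints clamped to MaxPoints, and plays a 2D sound.
; Pickup is disabled only when the player leaves the Box, then re-enabled with the Shape shown again after a Duration delay.
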(event OnComponentBeginOverlap(Box)
  (params (OverlappedComponent :type Primitive%20Component%20Object%20Reference) (OtherActor :type Actor%20Object%20Reference) (OtherComp :type Primitive%20Component%20Object%20Reference) (OtherBodyIndex :type Integer) (bFromSweep :type Boolean) (SweepResult :type Hit%20Result%20Structure%20%28by%20ref%29))
  (bind _playerref (Variables|Default|GetPlayerRef))
  ;[0.15 0.15 0.15 0.5] Pickup/turn off
  (if (and (== OtherActor (Game|GetPlayerCharacter 0)) (Variables|Default|GetCanPickUp?))
    (Rendering|SetVisibility (Variables|Default|GetShape) false false)
    (Variables|/Game/ThirdPerson/Blueprints/BP_ThirdPersonCharacter.BP_ThirdPersonCharacter_C|SetCurrentPoints _playerref (Math|Float|Clamp(Float) (+ (Variables|/Game/ThirdPerson/Blueprints/BP_ThirdPersonCharacter.BP_ThirdPersonCharacter_C|GetCurrentPoints _playerref) (Variables|Default|GetCustomScore)) 0.0 (Variables|/Game/ThirdPerson/Blueprints/BP_ThirdPersonCharacter.BP_ThirdPersonCharacter_C|GetMaxPoints _playerref)))
    (Audio|PlaySound2D "/Engine/VREditor/Sounds/UI/Dockable_Window_Pick_Up.Dockable_Window_Pick_Up" 1.0 1.0 0.0 0 0)))

(event OnComponentEndOverlap(Box)
  (params (OverlappedComponent :type Primitive%20Component%20Object%20Reference) (OtherActor :type Actor%20Object%20Reference) (OtherComp :type Primitive%20Component%20Object%20Reference) (OtherBodyIndex :type Integer))
  ;[0.15 0.15 0.15 0.5] Pickup/turn off
  (if (== OtherActor (Game|GetPlayerCharacter 0))
    (Variables|Default|SetCanPickUp? false)
    (Utilities|FlowControl|Delay (Variables|Default|GetDuration))
    (Variables|Default|SetCanPickUp? true)
    (Rendering|SetVisibility (Variables|Default|GetShape) true false)))

(event EventBeginPlay
  ;[0.15 0.15 0.15 0.5] Player Ref
  (bind _asbp_third_person_character (Utilities|Casting|CastToBP_ThirdPersonCharacter (Game|GetPlayerCharacter 0)))
  (Variables|Default|SetPlayerRef _asbp_third_person_character))

(fn ConstructionScript)