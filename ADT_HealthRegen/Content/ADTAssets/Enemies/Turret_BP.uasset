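; Enemy turret Blueprint that fires Bullet_BP projectiles in bursts of random length.
; A fast looping timer started at BeginPlay drives the FIRE event, with Delay nodes pacing the shots.
; While SHOOT is true it spawns bullets at its Arrow transform, passing itself as Enemy, and randomly clears the flag after a shot.
; When the flag is off, it pauses before resuming fire.
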(event Custom|FIRE
  ;[0.15 0.15 0.15 0.5] TurretShoot.
  (if (Variables|Default|GetSHOOT)
    (Utilities|FlowControl|Delay 0.5)
    (Game|SpawnActorfromClass "/Game/ADTAssets/Enemies/Bullet_BP.Bullet_BP_C" (Transformation|GetWorldTransform (Variables|Default|GetArrow)) "Undefined" "MultiplyWithRoot" 0 self 0)
    (if (== (Math|Random|RandomIntegerinRange 0 5) 3)
      (Variables|Default|SetSHOOT false))
    (else
      (Utilities|FlowControl|Delay 3.0)
      (Variables|Default|SetSHOOT true))))

(event EventBeginPlay
  ;[0.15 0.15 0.15 0.5] TurretShoot.
  (Utilities|Time|SetTimerbyEvent (delegate Custom|FIRE) 0.01 true))

(fn ConstructionScript)