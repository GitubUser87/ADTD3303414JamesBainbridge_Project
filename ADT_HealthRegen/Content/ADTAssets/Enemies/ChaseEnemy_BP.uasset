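; Chasing enemy that pursues the player, fires Bullet_BP projectiles and awards points when killed.
; BeginPlay caches the player, turns toward them once and starts FollowPlayer, which triggers delayed shots and AI movement, repeating after each successful move.
; A DangerZone overlap applies repeated contact damage while the player stays inside.
; The player's Safe flag clears on spawn and returns after a short delay or on destruction.
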(event OnComponentBeginOverlap(DangerZone)
  (params (OverlappedComponent :type Primitive%20Component%20Object%20Reference) (OtherActor :type Actor%20Object%20Reference) (OtherComp :type Primitive%20Component%20Object%20Reference) (OtherBodyIndex :type Integer) (bFromSweep :type Boolean) (SweepResult :type Hit%20Result%20Structure%20%28by%20ref%29))
  (bind _returnvalue (Game|GetPlayerCharacter 0))
  ;[1 0 0 0.5] DangerZone Overlap deal damage to player
  (if (== OtherActor _returnvalue)
    (Variables|Default|SetDanger true)
    (Game|Damage|ApplyDamage _returnvalue 1e+01 0 0 :!label _label)
    (Utilities|FlowControl|Delay 0.5)
    (if (Variables|Default|GetDanger)
      (goto _label))))

(event OnComponentEndOverlap(DangerZone)
  (params (OverlappedComponent :type Primitive%20Component%20Object%20Reference) (OtherActor :type Actor%20Object%20Reference) (OtherComp :type Primitive%20Component%20Object%20Reference) (OtherBodyIndex :type Integer))
  ;[1 0 0 0.5] DangerZone Overlap deal damage to player
  (if (== OtherActor (Game|GetPlayerCharacter 0))
    (Variables|Default|SetDanger false)))

(event Custom|Add%20Points
  (bind _charref (Variables|Default|GetCharREF))
  ;[0 0.15 0.003322 0.5] Add Points to the player upon death
  (if (!= (Variables|/Game/ThirdPerson/Blueprints/BP_ThirdPersonCharacter.BP_ThirdPersonCharacter_C|GetCurrentPoints _charref) 100)
    (Variables|/Game/ThirdPerson/Blueprints/BP_ThirdPersonCharacter.BP_ThirdPersonCharacter_C|SetCurrentPoints _charref (Math|Conversions|ToFloat(Integer) (Math|Integer|Clamp(Integer) (Math|Float|Truncate (+ (Variables|/Game/ThirdPerson/Blueprints/BP_ThirdPersonCharacter.BP_ThirdPersonCharacter_C|GetCurrentPoints _charref) (Variables|Default|GetPoints%20Earned))) 0 (Math|Float|Truncate (Variables|/Game/ThirdPerson/Blueprints/BP_ThirdPersonCharacter.BP_ThirdPersonCharacter_C|GetMaxPoints _charref)))))))

(event Custom|FollowPlayer
  ;[0.04673 0 0.15 0.5] Move to player + Shoot
  (Utilities|FlowControl|Sequence
    (:then_0
      (CallFunction|FIRE!))
    (:then_1
      (AI|AIMoveTo self "0, 0, 0" (Game|GetPlayerCharacter 0) 7e+01 false
        (:OnSuccess
          (Utilities|FlowControl|Delay 0.5)
          (CallFunction|FollowPlayer))))))

(event Custom|FIRE!
  ;[0.15 0.1446 0 0.5] Look at player & shoot
  (Utilities|FlowControl|Delay 2.0)
  (Game|SpawnActorfromClass "/Game/ADTAssets/Enemies/Bullet_BP.Bullet_BP_C" (Transformation|GetWorldTransform (Variables|Default|GetFire)) "Undefined" "MultiplyWithRoot" 0 self 0))

(event EventDestroyed
  ;[0 0.15 0.09462 0.5] When DEAD tell player they are safe.
  (Variables|/Game/ThirdPerson/Blueprints/BP_ThirdPersonCharacter.BP_ThirdPersonCharacter_C|SetSafe? (Variables|Default|GetCharREF) true))

(event Game|Damage|EventAnyDamage
  (params (Damage :type Float%20%28single-precision%29) (DamageType :type Damage%20Type%20Object%20Reference) (InstigatedBy :type Controller%20Object%20Reference) (DamageCauser :type Actor%20Object%20Reference))
  ;[1 0 0 0.5] Take Damage
  (bind _output_get (Variables|Default|SetHealth (- (Variables|Default|GetHealth) Damage)))
  (if (< _output_get 1.0)
    (CallFunction|AddPoints)
    (Actor|DestroyActor)))

(event EventBeginPlay
  ;[0.15 0.15 0.15 0.5] Player REF
  (bind _asbp_third_person_character (Utilities|Casting|CastToBP_ThirdPersonCharacter (Game|GetPlayerCharacter 0)))
  (Variables|Default|SetCharREF _asbp_third_person_character)
  ;[0.15 0.1446 0 0.5] Look at player & shoot
  (Utilities|FlowControl|Sequence
    (:then_0
      (Variables|/Game/ThirdPerson/Blueprints/BP_ThirdPersonCharacter.BP_ThirdPersonCharacter_C|SetSafe? (Variables|Default|GetCharREF) false)
      (Transformation|SetActorRotation (Math|Rotator|MakeRotator 0.0 0.0 (.yaw (Math|Interpolation|RInterpTo (Transformation|GetActorRotation) (Math|Rotator|FindLookatRotation (Transformation|GetActorLocation) (Transformation|GetActorLocation (Variables|Default|GetCharREF))) (Utilities|Time|GetWorldDeltaSeconds) (* 2e+01 5.0)))))
      (CallFunction|FollowPlayer))
    (:then_1
      (Utilities|FlowControl|RetriggerableDelay 0.6)
      (Variables|/Game/ThirdPerson/Blueprints/BP_ThirdPersonCharacter.BP_ThirdPersonCharacter_C|SetSafe? (Variables|Default|GetCharREF) true))))

(fn ConstructionScript)