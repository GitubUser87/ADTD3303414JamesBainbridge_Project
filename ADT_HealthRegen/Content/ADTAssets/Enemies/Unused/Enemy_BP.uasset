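; Enemy that turns toward, shoots and chases the player on sight, and dies from any damage.
; PawnSensing drives a yaw turn, a delayed Bullet_BP spawn from the Fire component, and a repeating AI MoveTo.
; Sightings clear the player's Safe flag, which a retriggerable delay restores once sightings stop, as does the enemy's destruction.
; Damage awards clamped points to the cached player character before destroying the enemy.
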(event OnSeePawn(PawnSensing)
  (params (Pawn :type Pawn%20Object%20Reference))
  (bind _charref (Variables|Default|GetCharREF))
  ;[0.15 0.15 0.15 0.5] Look at player & shoot
  (Utilities|FlowControl|Sequence
    (:then_0
      (Variables|/Game/ThirdPerson/Blueprints/BP_ThirdPersonCharacter.BP_ThirdPersonCharacter_C|SetSafe? _charref false)
      (Transformation|SetActorRotation (Math|Rotator|MakeRotator 0.0 0.0 (.yaw (Math|Interpolation|RInterpTo (Transformation|GetActorRotation) (Math|Rotator|FindLookatRotation (Transformation|GetActorLocation) (Transformation|GetActorLocation _charref)) (Utilities|Time|GetWorldDeltaSeconds) (* 2e+01 5.0)))))
      (Utilities|FlowControl|Delay 0.5)
      (Game|SpawnActorfromClass "/Game/ADTAssets/Enemies/Bullet_BP.Bullet_BP_C" (Transformation|GetWorldTransform (Variables|Default|GetFire)) "Undefined" "MultiplyWithRoot" 0 self 0)
      (AI|AIMoveTo self "0, 0, 0" (Game|GetPlayerCharacter 0) 5.0 false :!label _label
        (:OnSuccess
          (Utilities|FlowControl|Delay 0.2)
          (goto _label))))
    (:then_1
      (Utilities|FlowControl|RetriggerableDelay 0.6)
      (Variables|/Game/ThirdPerson/Blueprints/BP_ThirdPersonCharacter.BP_ThirdPersonCharacter_C|SetSafe? _charref true))))

(event Custom|Add%20Points
  (bind _charref (Variables|Default|GetCharREF))
  ;[0 0.15 0.003322 0.5] Add Points
  (if (!= (Variables|/Game/ThirdPerson/Blueprints/BP_ThirdPersonCharacter.BP_ThirdPersonCharacter_C|GetCurrentPoints _charref) 100)
    (Variables|/Game/ThirdPerson/Blueprints/BP_ThirdPersonCharacter.BP_ThirdPersonCharacter_C|SetCurrentPoints _charref (Math|Conversions|ToFloat(Integer) (Math|Integer|Clamp(Integer) (Math|Float|Truncate (+ (Variables|/Game/ThirdPerson/Blueprints/BP_ThirdPersonCharacter.BP_ThirdPersonCharacter_C|GetCurrentPoints _charref) (Variables|Default|GetPoints%20Earned))) 0 (Math|Float|Truncate (Variables|/Game/ThirdPerson/Blueprints/BP_ThirdPersonCharacter.BP_ThirdPersonCharacter_C|GetMaxPoints _charref)))))))

(event EventDestroyed
  ;[0.15 0.15 0.15 0.5] DEAD
  (Variables|/Game/ThirdPerson/Blueprints/BP_ThirdPersonCharacter.BP_ThirdPersonCharacter_C|SetSafe? (Variables|Default|GetCharREF) true))

(event Game|Damage|EventAnyDamage
  (params (Damage :type Float%20%28single-precision%29) (DamageType :type Damage%20Type%20Object%20Reference) (InstigatedBy :type Controller%20Object%20Reference) (DamageCauser :type Actor%20Object%20Reference))
  ;[1 0 0 0.5] Add Damage
  (CallFunction|AddPoints)
  (Actor|DestroyActor))

(event EventBeginPlay
  ;[0.15 0.15 0.15 0.5] Player REF
  (bind _asbp_third_person_character (Utilities|Casting|CastToBP_ThirdPersonCharacter (Game|GetPlayerCharacter 0)))
  (Variables|Default|SetCharREF _asbp_third_person_character))

(fn ConstructionScript)